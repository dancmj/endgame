(fn `Get Vertex Position`
  (params (Angle :type "Float (double-precision)"))
  (returns (`Vertex Location` :type "Vector Structure"))
  (bind (_vertex_p_location_x _vertex_p_location_y _vertex_p_location_z) (`KismetMathLibrary.BreakVector` (`self.Vertex P`)))
  (bind _radius (`self.radius`))
  (return (`KismetMathLibrary.MakeVector` (+ (* _radius (`KismetMathLibrary.DegCos` Angle)) _vertex_p_location_x) (+ (* _radius (`KismetMathLibrary.DegSin` Angle)) _vertex_p_location_y) _vertex_p_location_z)))

(fn `Make`
  (params (Radius :type Integer))
  (bind _proceduralmesh (`self.ProceduralMesh`))
  (set `self.radius` Radius)
  (`ProceduralMeshComponent.CreateMeshSection_LinearColor` :`self` _proceduralmesh :`Vertices` (`|MakeArray` (`self.Vertex P`) (`self.Vertex A`) (`self.Vertex B`) (`self.Vertex C`) (`self.Vertex D`) (`self.Vertex E`) (`self.Vertex F`)) :`Triangles` (`|MakeArray` 2 1 0 3 2 0 4 3 0 5 4 0 6 5 0 1 6 0))
  (`PrimitiveComponent.SetMaterial` _proceduralmesh 0 "/Engine/MapTemplates/Materials/BasicAsset01.BasicAsset01"))

(fn `UserConstructionScript`)

(fn `Vertex A`
  (returns (`Vector A Location` :type "Vector Structure"))
  (bind (_vertex_p_location_x _vertex_p_location_y _vertex_p_location_z) (`KismetMathLibrary.BreakVector` (`self.Vertex P`)))
  (return (`KismetMathLibrary.MakeVector` (+ (`KismetMathLibrary.Conv_IntToDouble` (`self.radius`)) _vertex_p_location_x) _vertex_p_location_y _vertex_p_location_z)))

(fn `Vertex B`
  (returns (`Vertex B Location` :type "Vector Structure"))
  (locals (`Vertex Angle` :type "Float (double-precision)" :default 60.0))
  (return (`self.Get Vertex Position` (`local.Vertex Angle`))))

(fn `Vertex C`
  (returns (`Vertex C Location` :type "Vector Structure"))
  (locals (`Vertex Angle` :type "Float (double-precision)" :default 120.0))
  (return (`self.Get Vertex Position` (`local.Vertex Angle`))))

(fn `Vertex D`
  (returns (`Vertex D Location` :type "Vector Structure"))
  (bind (_vertex_p_location_x _vertex_p_location_y _vertex_p_location_z) (`KismetMathLibrary.BreakVector` (`self.Vertex P`)))
  (return (`KismetMathLibrary.MakeVector` (+ (`KismetMathLibrary.Conv_IntToDouble` (* (`self.radius`) -1)) _vertex_p_location_x) _vertex_p_location_y _vertex_p_location_z)))

(fn `Vertex E`
  (returns (`Vertex E Location` :type "Vector Structure"))
  (locals (`Vertex Angle` :type "Float (double-precision)" :default 240.0))
  (return (`self.Get Vertex Position` (`local.Vertex Angle`))))

(fn `Vertex F`
  (returns (`Vertex F Location` :type "Vector Structure"))
  (locals (`Vertex Angle` :type "Float (double-precision)" :default 300.0))
  (return (`self.Get Vertex Position` (`local.Vertex Angle`))))

(fn `Vertex P`
  (returns (`Vertex P Location` :type "Vector Structure"))
  (return (0.0 0.0 0.0)))