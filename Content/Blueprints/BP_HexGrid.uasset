(fn `Make Grid`
  (locals (Q :type Integer) (R :type Integer))
  (bind _separation (`self.Separation`))
  (bind _hextable (`self.hexTable`))
  (bind _r (`local.R`))
  ;[0.6641 1 0] Setup
  (bind _values (`BlueprintMapLibrary.Map_Values` (`self.Tile Map`)))
  (for _array_element _values
    (`self.K2_DestroyActor` _array_element))
  (`HexTable.ClearMap` _hextable)
  (`self.CreateGrid` "Hexagon" (`self.map_radius`))
  (`BlueprintMapLibrary.Map_Clear` (`self.Tile Map`))
  (bind _returnvalue (`HexTable.GetHexCoordinates` _hextable))
  (for _array_element_2 _returnvalue
    (set `local.Q` (break `IntVector` _array_element_2))
    (set `local.R` (`.Y` (break `IntVector` _array_element_2)))
    (bind _returnvalue_2 (`|SpawnActorFromClass` (`self.TileClass`) (`KismetMathLibrary.MakeTransform` (`KismetMathLibrary.MakeVector` (+ (* (`local.Q`) _separation) (* _r (/ _separation 2.0))) (/ (* _r _separation) 3.465))) "Undefined" "OverrideRootScale" null null))
    (bind _asbp_hex_tile (cast `/Game/Blueprints/BP_HexTile` _returnvalue_2))
    (`Tile.Initialize` _asbp_hex_tile (`local.Q`) (`local.R`))
    (`BlueprintMapLibrary.Map_Add` (`self.Tile Map`) (`Tile.GetKey` _asbp_hex_tile) _asbp_hex_tile)
    (`/Game/Blueprints/BP_HexTile.Make` _asbp_hex_tile (`self.hex_radius`))))

(fn `UserConstructionScript`)